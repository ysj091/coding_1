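; Test actor Blueprint in a developer folder that endlessly flips its mesh material between a red and a purple glow every half second.
; The Construction Script creates a dynamic material instance on the static mesh's first slot and stores it as MICube.
; From BeginPlay, two custom events set GlowColor and toggle Rough Max, then call each other after a Delay to form the loop.
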(event Custom|빨간색으로
  (bind _mi_cube (Variables|Default|GetMI_cube))
  (Rendering|Material|SetVectorParameterValue _mi_cube "GlowColor" "(R=1.000000,G=0.100000,B=0.100000,A=1.000000)" :!class /Script/Engine.MaterialInstanceDynamic)
  (Rendering|Material|SetScalarParameterValue _mi_cube "Rough Max" 1.0 :!class /Script/Engine.MaterialInstanceDynamic)
  (Utilities|FlowControl|Delay 0.5)
  (CallFunction|보라색으로))

(event Custom|보라색으로
  (bind _mi_cube (Variables|Default|GetMI_cube))
  (Rendering|Material|SetVectorParameterValue _mi_cube "GlowColor" "(R=1.000000,G=0.000000,B=0.900000,A=1.000000)" :!class /Script/Engine.MaterialInstanceDynamic)
  (Rendering|Material|SetScalarParameterValue _mi_cube "Rough Max" 0.0 :!class /Script/Engine.MaterialInstanceDynamic)
  (Utilities|FlowControl|Delay 0.5)
  (CallFunction|빨간색으로))

(event EventBeginPlay
  (CallFunction|빨간색으로))

(event Collision|EventActorBeginOverlap
  (params (OtherActor :type Actor%20Object%20Reference)))

(event EventTick
  (params (DeltaSeconds :type Float%20%28single-precision%29)))

(fn ConstructionScript
  (bind _returnvalue (Rendering|Material|CreateDynamicMaterialInstance (Variables|Default|GetStaticMesh) 0 0 "None" :!class /Script/Engine.PrimitiveComponent))
  (Variables|Default|SetMI_cube _returnvalue))