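; Developer actor Blueprint that makes a static mesh continuously alternate between two color schemes once play begins.
; The construction script creates dynamic material instances for the mesh's first two material slots.
; Two custom events, "to red" and "to green" (Korean names), set tint vector parameters on both instances, then call each other after a one-second Delay, forming an endless loop without Tick.
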(event Custom|빨간색으로
  (Rendering|Material|SetVectorParameterValue (Variables|Default|GetMI_capcule1) "Color_Tint_R" "(R=1.000000,G=0.000000,B=0.000000,A=1.000000)" :!class /Script/Engine.MaterialInstanceDynamic)
  (Rendering|Material|SetVectorParameterValue (Variables|Default|GetMI_capcule2) "Color_Tint_B" "(R=0.000000,G=0.000000,B=1.000000,A=1.000000)" :!class /Script/Engine.MaterialInstanceDynamic)
  (Utilities|FlowControl|Delay 1.0)
  (CallFunction|녹색으로))

(event Custom|녹색으로
  (Rendering|Material|SetVectorParameterValue (Variables|Default|GetMI_capcule1) "Color_Tint_R" "(R=0.000000,G=1.000000,B=0.000000,A=1.000000)" :!class /Script/Engine.MaterialInstanceDynamic)
  (Rendering|Material|SetVectorParameterValue (Variables|Default|GetMI_capcule2) "Color_Tint_B" "(R=0.000000,G=1.000000,B=0.987353,A=1.000000)" :!class /Script/Engine.MaterialInstanceDynamic)
  (Utilities|FlowControl|Delay 1.0)
  (CallFunction|빨간색으로))

(event EventBeginPlay
  (CallFunction|빨간색으로))

(event Collision|EventActorBeginOverlap
  (params (OtherActor :type Actor%20Object%20Reference)))

(event EventTick
  (params (DeltaSeconds :type Float%20%28single-precision%29)))

(fn ConstructionScript
  (bind _returnvalue (Rendering|Material|CreateDynamicMaterialInstance (Variables|Default|GetStaticMesh) 0 0 "None" :!class /Script/Engine.PrimitiveComponent))
  (Variables|Default|SetMI_capcule2 _returnvalue)
  (bind _returnvalue_2 (Rendering|Material|CreateDynamicMaterialInstance (Variables|Default|GetStaticMesh) 1 0 "None" :!class /Script/Engine.PrimitiveComponent))
  (Variables|Default|SetMI_capcule1 _returnvalue_2))